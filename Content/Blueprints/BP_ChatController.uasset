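; Player controller for a turn-based multiplayer guessing game played through chat, managing each player's UI.
; It swaps between lobby, chat and result widgets, with lobby entry marked as called from C++.
; Events show ready players, toggle guess input with turn text, and display guess results and the winner or tie.
; Ready and reset requests go to BP_ChatModeBase via GetGameMode, while restart returns the player to the lobby.
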(event `EnableGuess`
  (params (bShouldEnable :type Boolean))
  (bind _chatwidget (`self.ChatWidget`))
  (`/Engine/EditorBlueprintResources/StandardMacros.IsValid` _chatwidget
    (:`Is Valid`
      (bind _aswbp_chat_widget (cast `/Game/Widgets/WBP_ChatWidget` _chatwidget))
      (`Widget.SetIsEnabled` (`ChatWidget.MessageTextBox` _aswbp_chat_widget) bShouldEnable)
      (if bShouldEnable
        (bind _turntext (`/Game/Widgets/WBP_ChatWidget.TurnText` _aswbp_chat_widget))
        (`TextBlock.SetText` _turntext "YOUR TURN")
        (else
          (`TextBlock.SetText` _turntext "Waiting for the opponent to make a guess..."))))))

(event `self.ReceiveBeginPlay`
  (if (`self.IsLocalController`)
    (bind _returnvalue (`|CreateWidget` "/Game/Widgets/WBP_LobbyWidget.WBP_LobbyWidget_C" self))
    (set `self.LobbyWidget` _returnvalue)))

(event `self.EnterLobbyWidget`
  (bind _lobbywidget (`self.LobbyWidget`))
  ; Called by C++ code
  (if (`KismetSystemLibrary.IsValid` (`self.LobbyWidget`))
    (`UserWidget.AddToViewport` _lobbywidget 0 :!label _label)
    (add `/Game/Widgets/WBP_LobbyWidget.PlayerReady` _lobbywidget (`|CreateDelegate` :!event `NotifyPlayerReady`))))

(event `EnterLobby`
  (if (not (`KismetSystemLibrary.IsValid` (`self.LobbyWidget`)))
    (bind _returnvalue (`|CreateWidget` "/Game/Widgets/WBP_LobbyWidget.WBP_LobbyWidget_C" self))
    (set `self.LobbyWidget` _returnvalue)
    (goto _label)))

(event `DisplayGuessResult`
  (params (InText :type Text))
  (bind _aswbp_chat_widget (cast `/Game/Widgets/WBP_ChatWidget` (`self.ChatWidget`)))
  (`TextBlock.SetText` (`/Game/Widgets/WBP_ChatWidget.InfoText` _aswbp_chat_widget) InText))

(event `EnterResultWidget`
  (if (`KismetSystemLibrary.IsValid` (`self.ChatWidget`))
    (`self.RemoveChatWidget`))
  (if (not (`KismetSystemLibrary.IsValid` (`self.ResultWidget`)))
    (bind _returnvalue (`|CreateWidget` "/Game/Widgets/WBP_ResultWidget.WBP_ResultWidget_C" self))
    (bind _output_get (set `self.ResultWidget` _returnvalue)))
  (`UserWidget.AddToViewport` _output_get 0)
  (add `Button.OnClicked` (`/Game/Widgets/WBP_ResultWidget.RestartButton` (`self.ResultWidget`)) (`|CreateDelegate` :!event `RequestRestart`)))

(event `NotifyPlayerReady`
  (bind _asbp_chat_mode_base (cast `/Game/GameModes/BP_ChatModeBase` (`GameplayStatics.GetGameMode`)))
  (`/Game/GameModes/BP_ChatModeBase.ServerPlayerReady` _asbp_chat_mode_base (`self.Username`))
  (`self.DisableReadyButton`))

(event `DisplayReadyPlayer`
  (params (ReadyUsername :type String))
  (if (`KismetSystemLibrary.IsValid` (`self.LobbyWidget`))
    (`/Game/Widgets/WBP_LobbyWidget.AddToReadyPlayerBox` (`self.LobbyWidget`) ReadyUsername)))

(event `DisplayWinner`
  (params (WinnerName :type String) (LoserName :type String) (bIsTie :type Boolean))
  (`self.EnterResultWidget`)
  (if bIsTie
    (`TextBlock.SetText` (`/Game/Widgets/WBP_ResultWidget.WinnerText` (`self.ResultWidget`)) (`|FormatText` "{name} TIE!" WinnerName))
    (`TextBlock.SetText` (`/Game/Widgets/WBP_ResultWidget.LoserText` (`self.ResultWidget`)) (`|FormatText` "{name} TIE!" LoserName))
    (else
      (`TextBlock.SetText` (`/Game/Widgets/WBP_ResultWidget.WinnerText` (`self.ResultWidget`)) (`|FormatText` "{name} WON!" WinnerName))
      (`TextBlock.SetText` (`/Game/Widgets/WBP_ResultWidget.LoserText` (`self.ResultWidget`)) (`|FormatText` "{name} LOST..." LoserName)))))

(event `DisableReadyButton`
  (if (`KismetSystemLibrary.IsValid` (`self.LobbyWidget`))
    (`Widget.SetIsEnabled` (`/Game/Widgets/WBP_LobbyWidget.ReadyButton` (`self.LobbyWidget`)) false)))

(event `ExitLobbyWidget`
  (if (`KismetSystemLibrary.IsValid` (`self.LobbyWidget`))
    (`Widget.RemoveFromParent` (`self.LobbyWidget`))
    (set `self.LobbyWidget` null)
    (`self.CreateChatWidget`)))

(event `RequestRestart`
  (`self.ExitResultWidget`)
  (`self.EnterLobby`))

(event `ServerReset`
  (bind _asbp_chat_mode_base (cast `/Game/GameModes/BP_ChatModeBase` (`GameplayStatics.GetGameMode`)))
  (`/Game/GameModes/BP_ChatModeBase.ResetGame` _asbp_chat_mode_base))

(event `ExitResultWidget`
  (if (`KismetSystemLibrary.IsValid` (`self.ResultWidget`))
    (`Widget.RemoveFromParent` (`self.ResultWidget`))
    (set `self.ResultWidget` null)))

(fn `UserConstructionScript`)